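; BP_GridGenerator builds a square grid of BP_BaseGridCell actors when play begins.
; InitializeGrid spawns GridSize squared cells row by row, placing each cell's mesh at world coordinates from its index times the mesh bounds, independent of the generator's location.
; Each cell gets GridMesh and query-and-physics collision on GameTraceChannel1 that blocks Pawns.
; An older construction-script version that added static mesh components is left disconnected.
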(event EventBeginPlay
  (CallFunction|InitializeGrid))

(fn ConstructionScript)

(fn InitializeGrid
  (bind _gridsize (Variables|Default|GetGridSize))
  (for _index (range 1 (* _gridsize _gridsize))
    (if (> (Variables|Default|GetX_Coord) (- (Variables|Default|GetGridSize) 1)) :!label _label
      (Variables|Default|SetX_Coord 0)
      (bind _result (Math|Integer|IncrementInt (Variables|Default|GetY_Coord))
        (:%20%20
          (Variables|Default|SetY_Coord _result)
          (goto _label)))
      (else
        (bind _returnvalue (Game|SpawnActorfromClass "/Game/_Project/Blueprints/GridCells/BP_BaseGridCell.BP_BaseGridCell_C" (Math|Transform|MakeTransform "0, 0, 0") "Undefined" "MultiplyWithRoot" 0 0))
        (Collision|SetCollisionObjectType (Variables|/Game/_Project/Blueprints/GridCells/BP_BaseGridCell.BP_BaseGridCell_C|GetGridCell _returnvalue) "ECC_GameTraceChannel1")
        (Collision|SetCollisionEnabled (Variables|/Game/_Project/Blueprints/GridCells/BP_BaseGridCell.BP_BaseGridCell_C|GetGridCell _returnvalue) "QueryAndPhysics")
        (Collision|SetCollisionResponsetoChannel (Variables|/Game/_Project/Blueprints/GridCells/BP_BaseGridCell.BP_BaseGridCell_C|GetGridCell _returnvalue) "ECC_Pawn" "ECR_Block")
        (Components|StaticMesh|SetStaticMesh (Variables|/Game/_Project/Blueprints/GridCells/BP_BaseGridCell.BP_BaseGridCell_C|GetGridCell _returnvalue) (Variables|Default|GetGridMesh))
        (Transformation|SetWorldLocation (Variables|/Game/_Project/Blueprints/GridCells/BP_BaseGridCell.BP_BaseGridCell_C|GetGridCell _returnvalue) (Math|Vector|MakeVector (* (.x (- (.Max (Components|StaticMesh|GetLocalBounds (Variables|/Game/_Project/Blueprints/GridCells/BP_BaseGridCell.BP_BaseGridCell_C|GetGridCell _returnvalue))) (.Min (Components|StaticMesh|GetLocalBounds (Variables|/Game/_Project/Blueprints/GridCells/BP_BaseGridCell.BP_BaseGridCell_C|GetGridCell _returnvalue))))) (Variables|Default|GetX_Coord)) (* (.y (- (.Max (Components|StaticMesh|GetLocalBounds (Variables|/Game/_Project/Blueprints/GridCells/BP_BaseGridCell.BP_BaseGridCell_C|GetGridCell _returnvalue))) (.Min (Components|StaticMesh|GetLocalBounds (Variables|/Game/_Project/Blueprints/GridCells/BP_BaseGridCell.BP_BaseGridCell_C|GetGridCell _returnvalue))))) (Variables|Default|GetY_Coord)) 0.0) false false)
        (bind _result_2 (Math|Integer|IncrementInt (Variables|Default|GetX_Coord))
          (:%20%20
            (Variables|Default|SetX_Coord _result_2)))))))