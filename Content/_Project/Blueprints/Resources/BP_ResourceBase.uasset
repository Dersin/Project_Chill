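; BP_ResourceBase is a base actor for resources, configured from the DAResource data asset.
; On BeginPlay, InitializeActor applies the asset's mesh to ResourceMesh, then caches its display name, drop item and amount range, interaction time and experience rate.
; The copy and Initialized flag depend on SetStaticMesh returning true; otherwise it only prints an error.
; The file holds no interaction or drop logic.
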(event EventBeginPlay
  (CallFunction|InitializeActor))

(fn ConstructionScript)

(fn InitializeActor
  (bind _da_resource (Variables|Default|GetDA_Resource))
  (bind _resource_struct (Variables|/Game/_Project/DataAssets/Resources/Core/PDA_ResourceData.PDA_ResourceData_C|GetResource_Struct _da_resource))
  (bind (_actorclass _display_name _actor_mesh _drop_item _min_amount _max_amount _interaction_time _experiencerate) (Utilities|Struct|BreakST_ResourceData _resource_struct))
  (bind _returnvalue (Components|StaticMesh|SetStaticMesh (Variables|Default|GetResourceMesh) _actor_mesh))
  (if _returnvalue
    (Variables|Default|SetDisplayName _display_name)
    (Variables|Default|SetItemToDrop _drop_item)
    (Variables|Default|SetDropMinAmount _min_amount)
    (Variables|Default|SetDropMaxAmount _max_amount)
    (Variables|Default|SetInteractionTime _interaction_time)
    (Variables|Default|SetExperienceRate _experiencerate)
    (Variables|Default|SetbInitialized true)
    (else
      (Development|PrintString "Mesh não foi inicializada"))))