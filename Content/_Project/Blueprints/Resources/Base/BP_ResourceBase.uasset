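; Base actor for resources, whose appearance is driven by a resource data asset.
; On BeginPlay it applies the mesh from the asset's resource struct to its mesh component, setting an Initialized flag on success or printing an error on failure.
; The TryInteract event is a placeholder that only prints a debug string.
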(event EventBeginPlay
  (CallFunction|InitializeActor))

(event EventTryInteract
  (Development|PrintString "aiiin interação"))

(fn ConstructionScript)

(fn InitializeActor
  (bind _returnvalue (Components|StaticMesh|SetStaticMesh (Variables|Default|GetResourceMesh) (.Actor_Mesh (Utilities|Struct|BreakST_ResourceData (Variables|/Game/_Project/DataAssets/Resources/Core/PDA_ResourceData.PDA_ResourceData_C|GetResource_Struct (Variables|Core|GetDA_Resource))))))
  (if _returnvalue
    (Variables|Core|SetbInitialized true)
    (else
      (Development|PrintString "Mesh não foi inicializada"))))