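; Actor component that stores an inventory of item quantities and owned tools.
; Items live in a map keyed by item, with functions to add, query, clear and remove, deleting entries whose amount drops to zero or below.
; New tools go into both a map and an array, which is searched for the highest-tier tool matching a required type and minimum tier.
; Debug prints report added items, failed lookups and the selected tool.
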(event EventBeginPlay)

(event EventTick
  (params (DeltaSeconds :type Float%20%28single-precision%29)))

(fn AddItem
  (params (Item_To_Add :type PDA%20Item%20Data%20Object%20Reference) (Quantity_To_Add :type Integer))
  (if (Utilities|Map|Contains (Variables|Default|GetItem_Map) Item_To_Add)
    (Utilities|Map|Add (Variables|Default|GetItem_Map) Item_To_Add (+ (Itens|GetQuantity Item_To_Add) Quantity_To_Add))
    (else
      (Utilities|Map|Add (Variables|Default|GetItem_Map) Item_To_Add Quantity_To_Add)))
  (Development|PrintString (Utilities|String|Append "Item:" (Utilities|String|ToString(Text) (.display_name (Variables|/Game/_Project/DataAssets/Itens/Core/PDA_ItemData.PDA_ItemData_C|GetItem_Struct Item_To_Add))) "Adicionado")))

(fn RemoveItemAmount
  (params (Item_To_Remove :type PDA%20Item%20Data%20Object%20Reference%20%28by%20ref%29) (Quantity_To_Remove :type Integer))
  (if (Itens|HasItem Item_To_Remove)
    (bind _output_get (LocalVariables|Set%20Current_Amount (Itens|GetQuantity Item_To_Remove)))
    (bind _output_get_2 (LocalVariables|SetNew_Amount (- _output_get Quantity_To_Remove)))
    (if (> _output_get_2 0)
      (Utilities|Map|Add (Variables|Default|GetItem_Map) Item_To_Remove (LocalVariables|GetNew_Amount))
      (else
        (Itens|RemoveItem Item_To_Remove)))))

(fn GetQuantity
  (params (Item_Key :type PDA%20Item%20Data%20Object%20Reference))
  (bind _item_map (Variables|Default|GetItem_Map))
  (bind (_value _returnvalue) (Utilities|Map|Find _item_map Item_Key))
  (if _returnvalue
    (return _value)
    (else
      (Development|PrintString (Utilities|String|Append "Item:" (Utilities|String|ToString(Text) (.Display_Name (Utilities|Struct|BreakST_ItemData (Variables|/Game/_Project/DataAssets/Itens/Core/PDA_ItemData.PDA_ItemData_C|GetItem_Struct Item_Key)))) "Nao Encontrado")))))

(fn ClearInventory
  (Utilities|Map|Clear (Variables|Default|GetItem_Map)))

(fn HasItem
  (params (Item_To_Find :type PDA%20Item%20Data%20Object%20Reference))
  (return (.ReturnValue (Utilities|Map|Find (Variables|Default|GetItem_Map) Item_To_Find))))

(fn RemoveItem
  (params (Item_To_Remove :type PDA%20Item%20Data%20Object%20Reference))
  (Utilities|Map|Remove (Variables|Default|GetItem_Map) Item_To_Remove))

(fn AddNewTool
  (params (Tool_To_Add :type PDA%20Tool%20Object%20Reference))
  (Utilities|Map|Add (Variables|Default|GetTools_Map) Tool_To_Add true)
  (Utilities|Array|Add (Variables|Default|GetOwned_Tools) Tool_To_Add))

(fn GetBestToolAvailable
  (params (RequiredToolType :type ETools%20Enum :default "NewEnumerator0") (RequiredToolTier :type ETiers%20Enum :default "NewEnumerator4"))
  (for _array_element (Variables|Default|GetOwned_Tools)
    (LocalVariables|SetOwnedToolType (.tool_type (Variables|/Game/_Project/DataAssets/Tools/Core/PDA_Tool.PDA_Tool_C|GetToolStructure _array_element)))
    (LocalVariables|SetOwnedToolTier (.tier (Variables|/Game/_Project/DataAssets/Tools/Core/PDA_Tool.PDA_Tool_C|GetToolStructure _array_element)))
    (if (Utilities|Enum|Equal(Enum) (LocalVariables|GetOwnedToolType) RequiredToolType)
      (if (>= (Math|Conversions|ToInteger(Byte) (LocalVariables|GetOwnedToolTier)) (Math|Conversions|ToInteger(Byte) RequiredToolTier))
        (if (> (Math|Conversions|ToInteger(Byte) (LocalVariables|GetOwnedToolTier)) (LocalVariables|GetBestTierInt))
          (LocalVariables|SetBestTierInt (Math|Conversions|ToInteger(Byte) (LocalVariables|GetOwnedToolTier)))
          (LocalVariables|SetBest_Tool _array_element)))))
  (Utilities|IsValid (LocalVariables|GetBest_Tool)
    (:Is%20Valid
      (Development|PrintString (Utilities|String|Append "melhor tool:" "" (Utilities|String|ToString(Name) (.tool_id (Variables|/Game/_Project/DataAssets/Tools/Core/PDA_Tool.PDA_Tool_C|GetToolStructure (LocalVariables|GetBest_Tool))))))
      (return (LocalVariables|GetBest_Tool)))))