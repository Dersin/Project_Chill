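; Actor component that tracks levels and experience for the skills listed in a skills data asset.
; On BeginPlay it fills a runtime map keyed by skill type, starting each skill at level 1 with its base XP threshold.
; Added XP can trigger several level-ups at once, each multiplying the threshold by the skill's growth factor and rounding it.
; XP accumulates without resetting; a test event and debug print remain.
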(event Custom|AddExpTest
  (CallFunction|AddExptoSkill "NewEnumerator8" 5e+02))

(event EventBeginPlay
  (CallFunction|InitializeSkills))

(fn InitializeSkills
  (for _array_element (Variables|/Game/_Project/DataAssets/Skills/Core/PDA_AllSkills.PDA_AllSkills_C|GetAllSkills (Variables|Default|GetDA_AllSkills))
    (Utilities|Map|Add (Variables|Default|GetRuntimeSkills) (Default|GetSkillType _array_element) (Utilities|Struct|MakeST_RunTimeSkillData _array_element 1 0.0 (Default|GetBaseExp _array_element)))))

(fn AddExptoSkill
  (params (SkillType :type ESkillType%20Enum :default "NewEnumerator0") (ExpToAdd :type Float%20%28double-precision%29))
  (bind _runtimeskills (Variables|Default|GetRuntimeSkills))
  (bind (_value _returnvalue) (Utilities|Map|Find _runtimeskills SkillType))
  (bind _output_get (LocalVariables|SetLocalRunTimeData _value))
  (if _returnvalue
    (bind _output_get_2 (LocalVariables|SetNewExpAmount (+ (.CurrentXP (Utilities|Struct|BreakST_RunTimeSkillData _output_get)) ExpToAdd)))
    (while (>= _output_get_2 (.XPToLevelUP (Utilities|Struct|BreakST_RunTimeSkillData _output_get)))
      (bind _result (Math|Integer|IncrementInt (CallFunction|GetCurrentLevel (LocalVariables|GetLocalRunTimeData)))
        (:%20%20
          (bind _output_get_3 (LocalVariables|SetLocalRunTimeData (Utilities|Struct|MakeST_RunTimeSkillData (.skill_data (LocalVariables|GetLocalRunTimeData)) _result (LocalVariables|GetNewExpAmount) (CallFunction|UpdateXptoLevelUp (.skill_data (LocalVariables|GetLocalRunTimeData)) (.xptolevelup (LocalVariables|GetLocalRunTimeData))))))
          (Utilities|Map|Add (Variables|Default|GetRuntimeSkills) SkillType _output_get_3)
          (Development|PrintString "Subi de nivel"))))
    (bind _output_get_4 (LocalVariables|SetLocalRunTimeData (Utilities|Struct|MakeST_RunTimeSkillData (.skill_data (LocalVariables|GetLocalRunTimeData)) (.currentlevel (LocalVariables|GetLocalRunTimeData)) (LocalVariables|GetNewExpAmount) (.xptolevelup (LocalVariables|GetLocalRunTimeData)))))
    (Utilities|Map|Add (Variables|Default|GetRuntimeSkills) SkillType _output_get_4)))

(fn UpdateXptoLevelUp
  (params (SkillData :type PDA%20Skill%20Data%20Object%20Reference) (CurrentExpToLevelUP :type Float%20%28double-precision%29))
  (return (Math|Conversions|ToFloat(Integer) (Math|Float|Round (* (Default|GetEXPGrowth SkillData) CurrentExpToLevelUP)))))

(fn GetCurrentLevel
  (params (RunTimeData :type ST%20Run%20Time%20Skill%20Data%20Structure))
  (return (.currentlevel RunTimeData)))