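; BP_BaseGridCell is a base grid cell actor that can randomly spawn a resource on itself.
; SpawnResource picks a random entry from ResourceSpawnList, rolls it against that resource's spawn percentage, then spawns its actor just above the cell mesh.
; A successful roll stores the spawned actor and flags the cell as occupied by a resource.
; A separate event applies SimpleMaterial to the cell, and GetReferences looks up the grid generator without storing it.
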(event Custom|SpawnResource
  (CallFunction|TrySpawnResource (CallFunction|PickResourcetoSpawn)))

(event Custom|setmaterial
  (Rendering|Material|SetMaterial (Variables|Default|GetGridCell) 0 "/Game/_Project/Blueprints/GridCells/SimpleMaterial.SimpleMaterial"))

(event EventBeginPlay)

(fn ConstructionScript)

(fn TrySpawnResource
  (params (ResourceToSpawn :type PDA%20Resource%20Data%20Object%20Reference))
  (bind _gridcell (Variables|Default|GetGridCell))
  (bind _returnvalue (Transformation|GetWorldLocation _gridcell))
  (if (<= (Math|Random|RandomIntegerinRange 1 100) (Default|GetResourceSpawnPercentage ResourceToSpawn))
    (bind _returnvalue_2 (Game|SpawnActorfromClass (Default|GetActorClass ResourceToSpawn) (Math|Transform|MakeTransform (Math|Vector|MakeVector (.x _returnvalue) (.y _returnvalue) (+ (.z _returnvalue) 5e+01)) "0, 0, 0" "1.000000,1.000000,1.000000") "Undefined" "MultiplyWithRoot" 0 0))
    (Variables|Resources|SetResourceActor_Ref _returnvalue_2)
    (Variables|Resources|SetbHasResource true)))

(fn GetReferences
  (Utilities|FlowControl|Sequence
    (:then_0
      (Actor|GetActorOfClass "/Game/_Project/Blueprints/GridGenerator/BP_GridGenerator.BP_GridGenerator_C"))))

(fn PickResourcetoSpawn
  (return (.OutItem (Utilities|Array|Random (Variables|/Game/_Project/DataAssets/GridCell/Core/PDA_GridAvailableResources.PDA_GridAvailableResources_C|GetResouces_Availables (Variables|Resources|GetResourceSpawnList))))))